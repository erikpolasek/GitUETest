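; Camera Blueprint that mirrors a tracked device's pose and offers keyboard nudging of its rig and lens.
; Each Tick copies the position and orientation of tracked device 1 onto the Tracker component's relative transform.
; Key-held Gates let Tick incrementally yaw the Scene component (Left), move it along world X (Up), or raise CineCamera focal length with a printout (Z).
; Adjustments run one way and per frame, without delta-time scaling.
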(event `self.ReceiveTick`
  (params (DeltaSeconds :type "Float (single-precision)"))
  (bind (_outposition _outorientation) (`SteamVRFunctionLibrary.GetTrackedDevicePositionAndOrientation` 1))
  (bind _tracker (`self.Tracker`))
  (`|ExecutionSequence`
    (:`then_0`
      (`SceneComponent.K2_SetRelativeRotation` _tracker _outorientation false false)
      (`SceneComponent.K2_SetRelativeLocation` _tracker _outposition false false))
    (:`then_1`
      (`/Engine/EditorBlueprintResources/StandardMacros.Gate` true :!label _label
        (:`Exit`
          (`self.cameraRotation`))))
    (:`then_2`
      (`/Engine/EditorBlueprintResources/StandardMacros.Gate` true :!label _label_2
        (:`Exit`
          (`self.cameraTranslation`))))
    (:`then_3`
      (`/Engine/EditorBlueprintResources/StandardMacros.Gate` true :!label _label_3
        (:`Exit`
          (`self.FOV`))))))

(event `Key|Left`
  (params (Key :type "Key Structure"))
  (:`Pressed`
    (goto _label :!via `Open`))
  (:`Released`
    (goto _label :!via `Close`)))

(event `Key|Up`
  (params (Key :type "Key Structure"))
  (:`Pressed`
    (goto _label_2 :!via `Open`))
  (:`Released`
    (goto _label_2 :!via `Close`)))

(event `Key|Z`
  (params (Key :type "Key Structure"))
  (:`Pressed`
    (goto _label_3 :!via `Open`))
  (:`Released`
    (goto _label_3 :!via `Close`)))

(fn `cameraRotation`
  (`SceneComponent.K2_SetRelativeRotation` (`self.Scene`) (`KismetMathLibrary.MakeRotator` 0.0 0.0 (+ (.yaw (`SceneComponent.RelativeRotation` (`self.Scene`))) 2.0)) false false))

(fn `cameraTranslation`
  (`SceneComponent.K2_SetWorldLocation` (`self.Scene`) (`KismetMathLibrary.MakeVector` (+ (.x (`SceneComponent.K2_GetComponentLocation` (`self.Scene`))) 10.0) (.y (`SceneComponent.K2_GetComponentLocation` (`self.Scene`))) (.z (`SceneComponent.K2_GetComponentLocation` (`self.Scene`)))) false false))

(fn `FOV`
  (bind _cinecamera (`self.CineCamera`))
  (bind _output_get (set `CineCameraComponent.CurrentFocalLength` (+ (`CineCameraComponent.CurrentFocalLength` _cinecamera) 1.0) _cinecamera))
  (`KismetSystemLibrary.PrintText` (`KismetTextLibrary.Conv_DoubleToText` _output_get "HalfToEven")))

(fn `UserConstructionScript`)